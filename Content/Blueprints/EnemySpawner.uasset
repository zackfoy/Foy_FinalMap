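; Trigger-driven enemy spawner actor that adds an Enemy_Character to the level when the player enters it.
; When its Box begins an overlap, it checks that the player character is overlapping the spawner, then counts every Enemy_Character in the level.
; If that count is below MaxEnemies, it spawns one AI enemy at a random point inside the SpawnVolume bounds.
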(event OnComponentBeginOverlap(Box)
  (params (OverlappedComponent :type Primitive%20Component%20Object%20Reference) (OtherActor :type Actor%20Object%20Reference) (OtherComp :type Primitive%20Component%20Object%20Reference) (OtherBodyIndex :type Integer) (bFromSweep :type Boolean) (SweepResult :type Hit%20Result%20Structure%20%28by%20ref%29))
  (if (Collision|IsOverlappingActor (Game|GetPlayerCharacter 0) (Components|GetOwner (Variables|Default|GetBox)) :!class /Script/Engine.Actor)
    (bind _outactors (Actor|GetAllActorsOfClass "/Game/Blueprints/Enemy_Character.Enemy_Character_C"))
    (if (< (Utilities|Array|Length _outactors) (Variables|Default|GetMaxEnemies))
      (AI|SpawnAIFromClass "/Game/Blueprints/Enemy_Character.Enemy_Character_C" 0 (Math|Random|RandomPointinBoundingBox (Transformation|GetWorldLocation (Variables|Default|GetSpawnVolume)) (Components|Box|GetScaledBoxExtent (Variables|Default|GetSpawnVolume))) "0, 0, 0" false 0))))

(event EventBeginPlay)

(event Collision|EventActorBeginOverlap
  (params (OtherActor :type Actor%20Object%20Reference)))

(event EventTick
  (params (DeltaSeconds :type Float%20%28single-precision%29)))

(fn ConstructionScript)